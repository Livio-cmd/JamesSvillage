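; Player controller that handles the player character's movement, mouse look and jump input, and shows the crosshair HUD.
; On BeginPlay it creates the HUD_CrossHair widget if no valid instance is stored, then adds it to the viewport.
; Input events drive player character 0 directly, with movement directions taken from control-rotation yaw only, so camera pitch does not affect them.
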(event Custom|Create%20CrossHair%20-%20HUD
  ;[1 1 1] Create CrossHair - HUD
  (Utilities|IsValid (Variables|Default|GetHUD%20-%20CH)
    (:Is%20Valid
      _)
    (:Is%20Not%20Valid
      (bind _returnvalue (UserInterface|CreateWidget "/Game/HUD/HUD_CrossHair.HUD_CrossHair_C"))
      (bind _output_get (Variables|Default|SetHUD%20-%20CH _returnvalue))))
  (UserInterface|Viewport|AddtoViewport _output_get 0))

(event EventBeginPlay
  ;[1 1 1] Init
  (CallFunction|CreateCrossHair-HUD))

(event Input|ActionEvents|InputActionJump
  (params (Key :type Key%20Structure :default "None"))
  (bind _returnvalue (Game|GetPlayerCharacter 0))
  ;[1 1 1] Jump - Input
  (:Pressed
    (Character|Jump _returnvalue))
  (:Released
    (Character|StopJumping _returnvalue)))

(event Input|AxisEvents|InputAxismoveF/B
  (params (AxisValue :type Float%20%28single-precision%29))
  ;[1 1 1] Player Movements - Input
  (Pawn|Input|AddMovementInput (Game|GetPlayerCharacter 0) (Math|Vector|GetForwardVector (Math|Rotator|MakeRotator 0.0 0.0 (.yaw (Pawn|GetControlRotation :!class /Script/Engine.Controller)))) AxisValue false))

(event Input|AxisEvents|InputAxismoveR/L
  (params (AxisValue :type Float%20%28single-precision%29))
  ;[1 1 1] Player Movements - Input
  (Pawn|Input|AddMovementInput (Game|GetPlayerCharacter 0) (Math|Vector|GetRightVector (Math|Rotator|MakeRotator 0.0 0.0 (.yaw (Pawn|GetControlRotation :!class /Script/Engine.Controller)))) AxisValue false))

(event Input|AxisEvents|InputAxisTurn
  (params (AxisValue :type Float%20%28single-precision%29))
  ;[1 1 1] Mouse - Input
  (Pawn|Input|AddControllerYawInput (Game|GetPlayerCharacter 0) AxisValue))

(event Input|AxisEvents|InputAxislookUp
  (params (AxisValue :type Float%20%28single-precision%29))
  ;[1 1 1] Mouse - Input
  (Pawn|Input|AddControllerPitchInput (Game|GetPlayerCharacter 0) AxisValue))

(fn ConstructionScript)