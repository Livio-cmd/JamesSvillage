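; BP_Vieux is an old-man quest-giver NPC who has the player collect wheels in exchange for a diamond.
; On BeginPlay he walks to the player, retrying on failure, then plays dialogue with input disabled.
; He then spawns wheels at every TargetPoint, shows a counter HUD and starts a looping timer to face the player.
; Box overlaps check the controller's wheel count, playing a reminder below four or a one-time success line and diamond spawn.
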(event OnComponentBeginOverlap(Box_Collider)
  (params (OverlappedComponent :type Primitive%20Component%20Object%20Reference) (OtherActor :type Actor%20Object%20Reference) (OtherComp :type Primitive%20Component%20Object%20Reference) (OtherBodyIndex :type Integer) (bFromSweep :type Boolean) (SweepResult :type Hit%20Result%20Structure%20%28by%20ref%29))
  ;[1 1 1] Close Of The Player
  (Utilities|Casting|CastToBP_Player OtherActor)
  (if (Variables|Default|GetIsMissionActive)
    (if (< (Variables|/Game/BluePrints/BP_PlayerController.BP_PlayerController_C|GetNumberOfWheels (Variables|Default|GetBP_PlayerController)) 4)
      (Audio|PlaySoundatLocation "/Game/Sounds/ou_sont_les_roues.ou_sont_les_roues" (Transformation|GetActorLocation) "0, 0, 0" 1.0 1.0 0.0 0 0 0)
      (else
        (Utilities|FlowControl|DoOnce false
          (:Completed
            (Audio|PlaySoundatLocation "/Game/Sounds/Mission_Vieux_Réussite.Mission_Vieux_Réussite" (Transformation|GetActorLocation) "0, 0, 0" 1.0 1.0 0.0 0 0 0)
            (Variables|Default|SetSpawnDiamond true)
            (CallFunction|SpawnDiamondFunction)
            (Widget|RemovefromParent (Variables|Default|GetNBRofWheel%20-%20hud))))))))

(event Custom|LookAtPlayer
  ;[1 1 1] Look At Player
  (Transformation|SetWorldRotation (Variables|Collision|GetCapsuleComponent) (Math|Conversions|RotationFromXVector (Transformation|GetActorLocation (Game|GetPlayerCharacter 0))) false false))

(event Custom|MoveToPlayer
  ;[1 1 1] Cinematique
  (AI|AIMoveTo self "0, 0, 0" (Game|GetPlayerCharacter 0) 1.5e+02 false
    (:OnSuccess
      (Input|DisableInput (Game|GetPlayerController 0) 0)
      (Audio|PlaySoundatLocation "/Game/Sounds/AudioMVieuxMonsieur.AudioMVieuxMonsieur" (Transformation|GetActorLocation) "0, 0, 0" 1.0 1.0 0.0 0 0 0)
      (Utilities|FlowControl|Delay 5.2)
      (Input|EnableInput (Game|GetPlayerController 0) 0)
      (CallFunction|SpawnWheel)
      (CallFunction|NBRofWheel-HUD)
      (Variables|Default|SetIsMissionActive true)
      (Utilities|Time|SetTimerbyFunctionName 0 "LookAtPlayer" 0.01 true))
    (:OnFail
      (CallFunction|MovetoPlayer))))

(event EventBeginPlay
  ;[1 1 1] Init
  (CallFunction|MovetoPlayer)
  (bind _returnvalue (Actor|GetActorOfClass "/Game/BluePrints/BP_PlayerController.BP_PlayerController_C"))
  (Variables|Default|SetBP_PlayerController _returnvalue))

(fn ConstructionScript)

(fn SpawnWheel
  (bind _outactors (Actor|GetAllActorsOfClass "/Script/Engine.TargetPoint"))
  (for _array_element _outactors
    (Game|SpawnActorfromClass "/Game/BluePrints/BluePrintsInGame/BP_Wheel.BP_Wheel_C" (Transformation|GetActorTransform _array_element) "AdjustIfPossibleButAlwaysSpawn" 0 0)))

(fn NBRofWheel-HUD
  (bind _returnvalue (UserInterface|CreateWidget "/Game/HUD/HUD_NBROfWheel.HUD_NBROfWheel_C"))
  (bind _output_get (Variables|Default|SetNBRofWheel%20-%20hud _returnvalue))
  (UserInterface|Viewport|AddtoViewport _output_get 0))

(fn SpawnDiamondFunction
  (Game|SpawnActorfromClass "/Game/BluePrints/BluePrintsInGame/BP_Diamond.BP_Diamond_C" (Transformation|GetActorTransform) "Undefined" 0 0))